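; BP_FishingCharacter is a fishing character Blueprint whose graph sets up positional voice chat.
; On BeginPlay, if a PlayerState is valid, it creates a VOIP talker, sets the mic threshold and attaches the voice to the capsule with fisherman attenuation.
; For the locally controlled character, console commands enable voice loopback and toggle speaking on.
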(event `self.ReceiveBeginPlay`
  (`self.InitializeVoiceChat`))

(event `InitializeVoiceChat`
  (bind _playerstate (`self.PlayerState`)
    (:`then`
      (bind _returnvalue (`VOIPTalker.CreateTalkerForPlayer` _playerstate))
      (set `self.VOIP` _returnvalue)
      (`VOIPStatics.SetMicThreshold` -1.0)
      (set `VOIPTalker.Settings` (make `VoiceSettings` (`self.CapsuleComponent`) "/Game/Movers/Characters/Fisherman/Audio/ATT_Fisherman_VOIP.ATT_Fisherman_VOIP") (`self.VOIP`))
      (if (`self.IsLocallyControlled`)
        (`KismetSystemLibrary.ExecuteConsoleCommand` "OSS.VoiceLoopback 1" null)
        (`KismetSystemLibrary.ExecuteConsoleCommand` "ToggleSpeaking 1" null)))
    (:`else`)))

(fn `UserConstructionScript`)