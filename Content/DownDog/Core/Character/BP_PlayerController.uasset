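; BP_PlayerController is the player controller that sets up input, HUD and the opening screen fade when play begins.
; BeginPlay sets the camera to a full black manual fade, adds the default and mouse-look Enhanced Input mapping contexts, and creates the W_HUD widget.
; After a short delay it starts a timed camera fade from full opacity to reveal the scene.
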(event `self.ReceiveBeginPlay`
  (`PlayerCameraManager.SetManualCameraFade` :`self` (`GameplayStatics.GetPlayerCameraManager` 0) :`InFadeAmount` 1.0)
  (`EnhancedInputSubsystemInterface.AddMappingContext` (subsystem `EnhancedInputLocalPlayerSubsystem`) "/Game/DownDog/Core/Input/IMC_Default.IMC_Default" 0 (struct))
  (`EnhancedInputSubsystemInterface.AddMappingContext` (subsystem `EnhancedInputLocalPlayerSubsystem`) "/Game/DownDog/Core/Input/IMC_MouseLook.IMC_MouseLook" 0 (struct))
  (bind _returnvalue (`|CreateWidget` "/Game/DownDog/UI/W_HUD.W_HUD_C"))
  (`UserWidget.AddToViewport` _returnvalue 0)
  (`KismetSystemLibrary.Delay` 0.5)
  (`PlayerCameraManager.StartCameraFade` :`self` (`GameplayStatics.GetPlayerCameraManager` 0) :`FromAlpha` 1.0 :`Duration` 1.5 :`bHoldWhenFinished` true))

(fn `UserConstructionScript`)